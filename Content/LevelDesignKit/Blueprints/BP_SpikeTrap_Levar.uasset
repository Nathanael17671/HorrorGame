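; Lever-operated spike trap that the player springs with the E key while the lever's trigger volume has input enabled.
; Any overlap with the volume enables input for player 0, and ending it disables input.
; E raises the spike mesh with a sound and flips the lever, then after the ResetTimes delay both snap back.
; An Activated flag blocks retriggering until the reset.
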(event `self.TV_Levar.OnComponentBeginOverlap`
  (params (OverlappedComponent :type "PrimitiveComponent Object Reference") (OtherActor :type "Actor Object Reference") (OtherComp :type "PrimitiveComponent Object Reference") (OtherBodyIndex :type Integer) (bFromSweep :type Boolean) (SweepResult :type "HitResult Structure (by ref)"))
  (`self.EnableInput` (`GameplayStatics.GetPlayerController` 0)))

(event `self.TV_Levar.OnComponentEndOverlap`
  (params (OverlappedComponent :type "PrimitiveComponent Object Reference") (OtherActor :type "Actor Object Reference") (OtherComp :type "PrimitiveComponent Object Reference") (OtherBodyIndex :type Integer))
  (`self.DisableInput` (`GameplayStatics.GetPlayerController` 0)))

(event `Key|E`
  (params (Key :type "Key Structure"))
  (:`Pressed`
    (if (not (`self.Activated`))
      (`|ExecutionSequence`
        (:`then_0`
          (set `self.Activated` true)
          (`AudioComponent.Play` (`self.SFX_SpikeApppear`) 0.0)
          (`SceneComponent.K2_SetRelativeLocation` (`self.SM_Spike`) (0.0 0.0 3.0) false false)
          (`KismetSystemLibrary.Delay` (`self.ResetTimes`))
          (`SceneComponent.K2_SetRelativeLocation` (`self.SM_Spike`) (0.0 0.0 -100.0) false false)
          (set `self.Activated` false)
          (`SceneComponent.K2_SetRelativeRotation` (`self.SM_LeverLarge`) (`KismetMathLibrary.MakeRotator` 0.0) false false))
        (:`then_1`
          (`SceneComponent.K2_SetRelativeRotation` (`self.SM_LeverLarge`) (`KismetMathLibrary.MakeRotator` 0.0 0.0 180.0) false false))))))

(fn `UserConstructionScript`)