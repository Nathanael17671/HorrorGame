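; BP_SpikeTrap is a trap actor that raises spikes shortly after something overlaps its trigger volume.
; An overlap on TV_Activate plays a warning sound, then after a short delay plays the spike sound and snaps the spike mesh up.
; After a hold it drops the mesh and re-arms, with an Activated flag blocking retriggers meanwhile.
; The graph filters no actors and applies no damage.
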(event `self.TV_Activate.OnComponentBeginOverlap`
  (params (OverlappedComponent :type "PrimitiveComponent Object Reference") (OtherActor :type "Actor Object Reference") (OtherComp :type "PrimitiveComponent Object Reference") (OtherBodyIndex :type Integer) (bFromSweep :type Boolean) (SweepResult :type "HitResult Structure (by ref)"))
  (if (not (`self.Activated`))
    (set `self.Activated` true)
    (`AudioComponent.Play` (`self.SFX_Warning`) 0.0)
    (`KismetSystemLibrary.Delay` 1.0)
    (`AudioComponent.Play` (`self.SFX_SpikeApppear`) 0.0)
    (`SceneComponent.K2_SetRelativeLocation` (`self.SM_Spike`) (0.0 0.0 3.0) false false)
    (`KismetSystemLibrary.Delay` 3.0)
    (`SceneComponent.K2_SetRelativeLocation` (`self.SM_Spike`) (0.0 0.0 -100.0) false false)
    (set `self.Activated` false)))

(fn `UserConstructionScript`)